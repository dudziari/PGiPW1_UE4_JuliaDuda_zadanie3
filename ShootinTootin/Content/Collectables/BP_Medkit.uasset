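; BP_Medkit is a health pickup that heals the BP_mrSHOOTIN character.
; When that character overlaps its Box, it adds HealthPickupAmount to Health, clamps the result between 0 and 100, and destroys itself.
; The guard before healing compares two constants rather than Health, so it always passes and the medkit is consumed even at full health.
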(event OnComponentBeginOverlap(Box)
  (params (OverlappedComponent :type Primitive%20Component%20Object%20Reference) (OtherActor :type Actor%20Object%20Reference) (OtherComp :type Primitive%20Component%20Object%20Reference) (OtherBodyIndex :type Integer) (bFromSweep :type Boolean) (SweepResult :type Hit%20Result%20Structure%20%28by%20ref%29))
  (bind _asbp_mr_shootin (Utilities|Casting|CastToBP_mrSHOOTIN OtherActor))
  (Variables|Default|SetAs%20BP%20Mr%20SHOOTIN _asbp_mr_shootin)
  (Variables|Default|SetHealth (Variables|/Game/Blueprints/BP_mrSHOOTIN.BP_mrSHOOTIN_C|GetHealth _asbp_mr_shootin))
  (if (not (== 0.0 1e+02))
    (Variables|/Game/Blueprints/BP_mrSHOOTIN.BP_mrSHOOTIN_C|SetHealth (Variables|Default|GetAs%20BP%20Mr%20SHOOTIN) (Math|Float|Clamp(Float) (+ (Variables|Default|GetHealth) (Variables|Default|GetHealth%20Pickup%20Amount)) 0.0 1e+02))
    (Actor|DestroyActor)))

(fn ConstructionScript)